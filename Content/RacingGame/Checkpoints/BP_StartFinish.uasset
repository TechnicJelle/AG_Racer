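; BP_StartFinish is the combined start and finish line trigger for the racing game.
; The first wheeled vehicle overlap of its TriggerBox sets Started and calls GameStart on GM_RacingGame, while Tick accumulates time since then.
; A later overlap calls WinCrossTheFinishLine only once that time exceeds the game mode's InitialTimerDuration.
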(event OnComponentBeginOverlap(TriggerBox)
  (params (OverlappedComponent :type Primitive%20Component%20Object%20Reference) (OtherActor :type Actor%20Object%20Reference) (OtherComp :type Primitive%20Component%20Object%20Reference) (OtherBodyIndex :type Integer) (bFromSweep :type Boolean) (SweepResult :type Hit%20Result%20Structure%20%28by%20ref%29))
  (bind _returnvalue (Game|GetGameMode))
  (Utilities|Casting|CastToWheeledVehiclePawn OtherActor)
  (if (Variables|Default|GetStarted)
    (if (> (Variables|Default|GetTimeStarted) (Variables|/Game/RacingGame/Framework/GM_RacingGame.GM_RacingGame_C|GetInitialTimerDuration (stale EventBeginPlay _asgm_racing_game)))
      (Development|PrintString "Passed finish line")
      (bind _asgm_racing_game (Utilities|Casting|CastToGM_RacingGame _returnvalue))
      (Default|WinCrosstheFinishLine _asgm_racing_game))
    (else
      (Variables|Default|SetStarted true)
      (Development|PrintString "Passed starting line")
      (bind _asgm_racing_game_2 (Utilities|Casting|CastToGM_RacingGame _returnvalue))
      (Default|GameStart _asgm_racing_game_2))))

(event EventBeginPlay
  (bind _asgm_racing_game (Utilities|Casting|CastToGM_RacingGame (Game|GetGameMode))))

(event EventTick
  (params (DeltaSeconds :type Float%20%28single-precision%29))
  (if (Variables|Default|GetStarted)
    (Variables|Default|SetTimeStarted (+ (Variables|Default|GetTimeStarted) DeltaSeconds))))

(fn ConstructionScript)