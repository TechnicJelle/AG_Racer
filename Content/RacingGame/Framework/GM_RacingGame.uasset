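; Racing game mode that runs a checkpoint time trial with win and lose outcomes.
; GameStart starts the countdown timer and binds to every BP_Checkpoint, whose crossings re-set the timer with added time and play a HUD animation.
; Timeout prints a loss and opens a restart widget with UI-only input.
; Crossing the finish line clears the timer and prints a win.
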(event Custom|Game%20Start
  (Development|PrintString "Game started")
  (bind _returnvalue (Utilities|Time|SetTimerbyEvent (delegate Custom|Lose_OutOfTime) (Variables|Default|GetInitialTimerDuration)))
  (Variables|Default|SetTimeRemainingTimer _returnvalue)
  (bind _outactors (Actor|GetAllActorsOfClass "/Game/RacingGame/Checkpoints/BP_Checkpoint.BP_Checkpoint_C"))
  (for _array_element _outactors
    (EventDispatchers|BindEventtoOnCheckpointCrossed _array_element (delegate Custom|CrossedCheckpoint))
    (Development|PrintString (Utilities|GetDisplayName _array_element))))

(event Custom|CrossedCheckpoint
  (params (WithTime :type Float%20%28double-precision%29))
  (CallFunction|AddTimetoTimer WithTime))

(event Custom|Game%20Finish
  (params (Win :type Boolean))
  (Development|PrintString (Utilities|String|SelectString "You win!" "You lose..." Win)))

(event Custom|Lose_OutOfTime
  (Development|PrintString "Out of Time")
  (CallFunction|GameFinish false)
  (bind _returnvalue (UserInterface|CreateWidget "/Game/RacingGame/UI/WBP_LoseRestart.WBP_LoseRestart_C"))
  (UserInterface|Viewport|AddtoViewport _returnvalue 0)
  (Input|SetInputModeUIOnly (Game|GetPlayerController 0) (Variables|/Game/RacingGame/UI/WBP_LoseRestart.WBP_LoseRestart_C|GetRestartButton _returnvalue) "DoNotLock" false))

(event Custom|Win_CrossTheFinishLine
  (Utilities|Time|ClearandInvalidateTimerbyHandle (Variables|Default|GetTimeRemainingTimer))
  (CallFunction|GameFinish true))

(event EventBeginPlay
  (Development|PrintString "In pre-race state")
  (Input|SetInputModeGameOnly (Game|GetPlayerController 0) false))

(fn ConstructionScript)

(fn AddTimetoTimer
  (params (TimeToAdd :type Float%20%28double-precision%29))
  (bind _returnvalue (Utilities|Time|SetTimerbyEvent (EventDispatchers|CreateEvent :!event Custom|Lose_OutOfTime) (+ TimeToAdd (Utilities|Time|GetTimerRemainingTimebyHandle (Variables|Default|GetTimeRemainingTimer)))))
  (Variables|Default|SetTimeRemainingTimer _returnvalue)
  (bind _asvehicle_player_controller (Utilities|Casting|CastToVehiclePlayerController (Game|GetPlayerController 0)))
  (Default|StartTimeAddedAnim (Variables|/Game/VehicleTemplate/Blueprints/VehiclePlayerController.VehiclePlayerController_C|GetVehicleHud _asvehicle_player_controller)))